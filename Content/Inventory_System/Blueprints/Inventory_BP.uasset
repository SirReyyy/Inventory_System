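; Inventory Blueprint that stores items as class and quantity pairs in a slot array sized on BeginPlay.
; Helper functions check slots, read item info from class defaults, and find empty slots or partial stacks.
; AddItem tops up stacks before using empty slots, recursing on overflow and ignoring whether that succeeds.
; Non-stackable items take one slot each, but recursion passes the quantity undecremented, so multiples fill every empty slot.
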(event `self.ReceiveBeginPlay`
  (`KismetArrayLibrary.Array_Resize` (`self.InventorySlots`) (`self.NumberOfSlots`)))

(fn `F AddItem`
  (params (ItemClass :type "/Game/Inventory_System/Blueprints/Item_Classes/Item_MasterBP Class Reference") (ItemQuantity :type Integer))
  (returns (Success :type Boolean))
  (locals (Local_ItemClass :type "/Game/Inventory_System/Blueprints/Item_Classes/Item_MasterBP Class Reference") (Local_ItemQuantity :type Integer) (Local_ItemIndex :type Integer :default 0))
  (bind _returnvalue (+ (`.Inv_ItemQuantity_6_DDC41CE44A02529C28370F931FBE5946` (break `/Game/Inventory_System/Blueprints/Structures/S_Inventory_Slot` (`|GetArrayItem` (`self.InventorySlots`) (`local.Local_ItemIndex`)))) (`local.Local_ItemQuantity`)))
  (set `local.Local_ItemClass` ItemClass)
  (set `local.Local_ItemQuantity` ItemQuantity)
  (if (`.Item_isStackable_18_B2D097134FCE038BA40764BC104A78F1` (break `/Game/Inventory_System/Blueprints/Structures/S_Item_Info` (defaults `Object` (`local.Local_ItemClass`))))
    (bind (_success _slotindex) (`self.F FindFreeStack` (`local.Local_ItemClass`)))
    (set `local.Local_ItemIndex` _slotindex)
    (if _success
      (if (> _returnvalue (`self.MaxStackSize`))
        (set `local.Local_ItemQuantity` (- _returnvalue (`self.MaxStackSize`)))
        (`KismetArrayLibrary.Array_Set` (`self.InventorySlots`) (`local.Local_ItemIndex`) (make `/Game/Inventory_System/Blueprints/Structures/S_Inventory_Slot` (`local.Local_ItemClass`) (`self.MaxStackSize`)))
        (`self.F AddItem` (`local.Local_ItemClass`) (`local.Local_ItemQuantity`))
        (return true)
        (else
          (`KismetArrayLibrary.Array_Set` (`self.InventorySlots`) (`local.Local_ItemIndex`) (make `/Game/Inventory_System/Blueprints/Structures/S_Inventory_Slot` (`local.Local_ItemClass`) _returnvalue))
          (return true)))
      (else
        (bind (_success_2 _slotindex_2) (`self.F FindEmptySlot`))
        (if _success_2
          (if (> (`local.Local_ItemQuantity`) (`self.MaxStackSize`))
            (`KismetArrayLibrary.Array_Set` (`self.InventorySlots`) _slotindex_2 (make `/Game/Inventory_System/Blueprints/Structures/S_Inventory_Slot` (`local.Local_ItemClass`)))
            (`self.F AddItem` (`local.Local_ItemClass`) (- (`local.Local_ItemQuantity`) (`self.MaxStackSize`)))
            (return true)
            (else
              (`KismetArrayLibrary.Array_Set` (`self.InventorySlots`) _slotindex_2 (make `/Game/Inventory_System/Blueprints/Structures/S_Inventory_Slot` (`local.Local_ItemClass`) (`local.Local_ItemQuantity`)))
              (return true)))
          (else
            (return false)))))
    (else
      (bind (_success_3 _slotindex_3) (`self.F FindEmptySlot`))
      (if _success_3
        (`KismetArrayLibrary.Array_Set` (`self.InventorySlots`) _slotindex_3 (make `/Game/Inventory_System/Blueprints/Structures/S_Inventory_Slot` (`local.Local_ItemClass`) 1))
        (if (> (`local.Local_ItemQuantity`) 1)
          (`self.F AddItem` (`local.Local_ItemClass`) (`local.Local_ItemQuantity`))
          (return true)
          (else
            (return true)))
        (else
          (return false))))))

(fn `F FindEmptySlot`
  (returns (Success :type Boolean) (SlotIndex :type Integer))
  (locals (Local_Bool :type Boolean) (Local_SlotIndex :type Integer))
  (for (_array_element _array_index) (`self.InventorySlots`)
    (if (not (`KismetSystemLibrary.IsValidClass` (`.Inv_ItemClass_7_C0520088489D9D81603D7B99C37CA198` (break `/Game/Inventory_System/Blueprints/Structures/S_Inventory_Slot` _array_element))))
      (set `local.Local_SlotIndex` _array_index)
      (set `local.Local_Bool` true)
      (break)))
  (return (`local.Local_Bool`) (`local.Local_SlotIndex`)))

(fn `F FindFreeStack`
  (params (ItemClass :type "/Game/Inventory_System/Blueprints/Item_Classes/Item_MasterBP Class Reference"))
  (returns (Success :type Boolean) (SlotIndex :type Integer))
  (locals (Local_ItemClass :type "/Game/Inventory_System/Blueprints/Item_Classes/Item_MasterBP Class Reference") (Local_Bool :type Boolean) (Local_SlotIndex :type Integer))
  (set `local.Local_ItemClass` ItemClass)
  (for (_array_element _array_index) (`self.InventorySlots`)
    (bind (_inv_itemclass _inv_itemquantity) (break `/Game/Inventory_System/Blueprints/Structures/S_Inventory_Slot` _array_element))
    (if (`KismetSystemLibrary.IsValidClass` _inv_itemclass)
      (if (and (== _inv_itemclass (`local.Local_ItemClass`)) (< _inv_itemquantity (`self.MaxStackSize`)))
        (set `local.Local_SlotIndex` _array_index)
        (set `local.Local_Bool` true)
        (break))))
  (return (`local.Local_Bool`) (`local.Local_SlotIndex`)))

(fn `F GetItemInfoAtIndex`
  (params (SlotIndex :type Integer))
  (returns (isEmpty :type Boolean) (ItemInfo :type "/Game/Inventory_System/Blueprints/Structures/S_Item_Info Structure") (ItemQuantity :type Integer))
  (locals (Local_SlotIndex :type Integer))
  (bind (_inv_itemclass _inv_itemquantity) (break `/Game/Inventory_System/Blueprints/Structures/S_Inventory_Slot` (`|GetArrayItem` (`self.InventorySlots`) (`local.Local_SlotIndex`))))
  (set `local.Local_SlotIndex` SlotIndex)
  (if (`KismetSystemLibrary.IsValidClass` _inv_itemclass)
    (return false (defaults `Object` _inv_itemclass) _inv_itemquantity)
    (else
      (return true (struct) 0))))

(fn `F isSlotEmpty`
  (params (SlotIndex :type Integer))
  (returns (isEmpty :type Boolean))
  (locals (Local_SlotIndex :type Integer))
  (set `local.Local_SlotIndex` SlotIndex)
  (return (not (`KismetSystemLibrary.IsValidClass` (`.Inv_ItemClass_7_C0520088489D9D81603D7B99C37CA198` (break `/Game/Inventory_System/Blueprints/Structures/S_Inventory_Slot` (`|GetArrayItem` (`self.InventorySlots`) (`local.Local_SlotIndex`))))))))

(fn `UserConstructionScript`)